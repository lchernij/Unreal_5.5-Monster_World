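; BP_Red is the player character Red, a top-down flipbook character that walks and picks up items.
; BeginPlay adds the Enhanced Input mapping context and creates the main HUD.
; Move input drives world-axis movement and stores direction, which UpdateAnimation uses to choose four-way walk or idle flipbooks, favoring horizontal.
; Interact picks a BP_Pickup overlapping InteractCheck, shows its item on the HUD, and hides the message after a retriggerable delay.
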(event Input|EnhancedActionEvents|EnhancedInputActionIA_Move
  (params (ActionValue :type Vector%202D%20Structure) (ElapsedSeconds :type Float%20%28double-precision%29) (TriggeredSeconds :type Float%20%28double-precision%29) (InputAction :type Input%20Action%20Object%20Reference :default "/Game/Dynamic/Input/Actions/IA_Move.IA_Move"))
  (bind (_x _y) (Math|Vector2D|BreakVector2D ActionValue))
  (:Triggered
    (Variables|Default|SetDirectionality ActionValue)
    (Pawn|Input|AddMovementInput "1.000000,0.000000,0.000000" _x false)
    (Pawn|Input|AddMovementInput "0.000000,1.000000,0.000000" _y false)
    (CallFunction|UpdateAnimation false))
  (:Completed
    (CallFunction|UpdateAnimation true)))

(event Input|EnhancedActionEvents|EnhancedInputActionIA_Interact
  (params (ActionValue :type Boolean) (ElapsedSeconds :type Float%20%28double-precision%29) (TriggeredSeconds :type Float%20%28double-precision%29) (InputAction :type Input%20Action%20Object%20Reference :default "/Game/Dynamic/Input/Actions/IA_Interact.IA_Interact"))
  (:Started
    (bind _array_element (Utilities|Array|ForEachLoopwithBreak (Collision|GetOverlappingActors (Variables|Default|GetInteractCheck) 0 :!class /Script/Engine.PrimitiveComponent) :!label _label)
      (:LoopBody
        (bind _asbp_pickup (Utilities|Casting|CastToBP_Pickup _array_element))
        (bind (_itemname _itemid) (Default|GetPicked _asbp_pickup))
        (Default|SetItemText (Variables|Default|GetMainHUD) _itemname _itemid)
        (goto _label Break))
      (:Completed
        (Utilities|FlowControl|RetriggerableDelay (Variables|Default|GetHideMessageDelay))
        (Default|HideMessage (Variables|Default|GetMainHUD))))))

(event EventBeginPlay
  (Utilities|FlowControl|Sequence
    (:then_0
      (bind _asplayer_controller (Utilities|Casting|CastToPlayerController (Pawn|GetController)))
      (Input|AddMappingContext (PlayerController|LocalPlayerSubsystems|GetEnhancedInputLocalPlayerSubsystem _asplayer_controller) "/Game/Dynamic/Input/IMC_TopDown.IMC_TopDown" 0 "(bIgnoreAllPressedKeysUntilRelease=True,bForceImmediately=False,bNotifyUserSettings=False)"))
    (:then_1
      (bind _returnvalue (UserInterface|CreateWidget "/Game/Dynamic/Widgets/WBP_MainHUD.WBP_MainHUD_C"))
      (UserInterface|Viewport|AddtoViewport _returnvalue 0)
      (Variables|Default|SetMainHUD _returnvalue))))

(event Collision|EventActorBeginOverlap
  (params (OtherActor :type Actor%20Object%20Reference)))

(event EventTick
  (params (DeltaSeconds :type Float%20%28single-precision%29)))

(fn ConstructionScript)

(fn UpdateAnimation
  (params (TransactionToIdle :type Boolean))
  (if TransactionToIdle
    (Math|Float|CompareFloat (.X (Math|Vector2D|BreakVector2D (Variables|Default|GetDirectionality))) 0.0
      (:>
        (Sprite|SetFlipbook (Variables|Default|GetSprite) "/Game/Static/PaperAssets/Characters/Red/FB_Red_Idle_R.FB_Red_Idle_R"))
      (:==
        (Math|Float|CompareFloat (.Y (Math|Vector2D|BreakVector2D (Variables|Default|GetDirectionality))) 0.0
          (:>
            (Sprite|SetFlipbook (Variables|Default|GetSprite) "/Game/Static/PaperAssets/Characters/Red/FB_Red_Idle_D.FB_Red_Idle_D"))
          (:<
            (Sprite|SetFlipbook (Variables|Default|GetSprite) "/Game/Static/PaperAssets/Characters/Red/FB_Red_Idle_U.FB_Red_Idle_U"))))
      (:<
        (Sprite|SetFlipbook (Variables|Default|GetSprite) "/Game/Static/PaperAssets/Characters/Red/FB_Red_Idle_L.FB_Red_Idle_L")))
    (else
      (Math|Float|CompareFloat (.X (Math|Vector2D|BreakVector2D (Variables|Default|GetDirectionality))) 0.0
        (:>
          (Sprite|SetFlipbook (Variables|Default|GetSprite) "/Game/Static/PaperAssets/Characters/Red/FB_Red_Walk_R.FB_Red_Walk_R"))
        (:==
          (Math|Float|CompareFloat (.Y (Math|Vector2D|BreakVector2D (Variables|Default|GetDirectionality))) 0.0
            (:>
              (Sprite|SetFlipbook (Variables|Default|GetSprite) "/Game/Static/PaperAssets/Characters/Red/FB_Red_Walk_D.FB_Red_Walk_D"))
            (:<
              (Sprite|SetFlipbook (Variables|Default|GetSprite) "/Game/Static/PaperAssets/Characters/Red/FB_Red_Walk_U.FB_Red_Walk_U"))))
        (:<
          (Sprite|SetFlipbook (Variables|Default|GetSprite) "/Game/Static/PaperAssets/Characters/Red/FB_Red_Walk_L.FB_Red_Walk_L"))))))